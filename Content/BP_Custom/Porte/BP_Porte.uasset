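; BP_Porte is a door that slides between its starting location and a target location, toggled by bullet hits.
; Each BulletHit calls PorteActive, where a FlipFlop alternately plays and reverses the OuverturePorte timeline and updates the Actif flag.
; The timeline's alpha lerps the actor's location from the base position cached at BeginPlay to TargetLocation.
; If Actif is set at BeginPlay, the door starts opening immediately.
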(event `self.ReceiveBeginPlay`
  (set `self.BaseLocation` (`self.K2_GetActorLocation` self))
  (if (`self.Actif`)
    (`self.PorteActive`)))

(event `/Game/BP_Interface/BPI_BulletHit.BulletHit`
  (`self.PorteActive`))

(event `PorteActive`
  (`/Engine/EditorBlueprintResources/StandardMacros.FlipFlop`
    (:`A`
      (set `self.Actif` true)
      (bind (_direction _alpha) (`Timeline|OuverturePorte` :!label _label)
        (:`Update`
          (`self.K2_SetActorLocation` (`KismetMathLibrary.VLerp` (`self.BaseLocation`) (`self.TargetLocation`) _alpha)))))
    (:`B`
      (set `self.Actif` false)
      (goto _label :!via `Reverse`))))

(fn `UserConstructionScript`)