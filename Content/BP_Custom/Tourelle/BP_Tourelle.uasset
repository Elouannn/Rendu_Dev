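; Turret that aims at the player and fires enemy projectiles, with an activator that toggles its active state and particle effect.
; Viser yaws the cylinder toward the player every frame through a gated delay loop while Actif is true.
; After a retriggerable delay, Tir spawns a projectile, closes the gate, then calls Viser again after a pause.
; This firing cycle does not itself check Actif.
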(event `self.ReceiveBeginPlay`
  ;[0.4334 1 0.3801] Initialisation
  (bind _asbp_first_person_character (cast `/Game/FirstPerson/Blueprints/BP_FirstPersonCharacter` (`GameplayStatics.GetPlayerCharacter` 0)))
  (set `self.Player` _asbp_first_person_character)
  (add `/Game/BP_Custom/LightActivable/BP_ActiveLight.StartAndStop` (`self.Activateur`) (delegate `ActiveDesactive`)))

(event `ActiveDesactive`
  ;[0.593 1 0] Activer/Désactiver la tourelle
  (bind _isa (`/Engine/EditorBlueprintResources/StandardMacros.FlipFlop`)
    (:`A`
      _)
    (:`B`
      _))
  (bind _output_get (set `self.Actif` _isa))
  (`SceneComponent.SetHiddenInGame` (`self.ParticleSystem`) (not _output_get) false)
  (`self.Viser`))

(event `Viser`
  (bind (_returnvalue_roll _returnvalue_pitch _returnvalue_yaw) (`KismetMathLibrary.BreakRotator` (`KismetMathLibrary.FindLookAtRotation` (`self.K2_GetActorLocation` self) (`self.K2_GetActorLocation` (`self.Player`)))))
  ;[1 0.4428 0] Visée et cooldown
  (`|ExecutionSequence`
    (:`then_0`
      (`/Engine/EditorBlueprintResources/StandardMacros.IsValid` (`self.Player`) :!label _label
        (:`Is Valid`
          (`SceneComponent.K2_SetWorldRotation` (`self.Cylinder`) (`KismetMathLibrary.MakeRotator` 0.0 0.0 _returnvalue_yaw) false false)
          (`KismetSystemLibrary.Delay` (`GameplayStatics.GetWorldDeltaSeconds`))
          (if (`self.Actif`)
            (`/Engine/EditorBlueprintResources/StandardMacros.Gate` false :!label _label_2
              (:`Exit`
                (goto _label)))))))
    (:`then_1`
      (goto _label_2 :!via `Open`))
    (:`then_2`
      (`KismetSystemLibrary.RetriggerableDelay` (`self.DelayPourTir`))
      (`self.Tir`)
      (goto _label_2 :!via `Close`))))

(event `Tir`
  ;[1 0 0.01854] Tir
  (`|SpawnActorFromClass` "/Game/FirstPerson/Blueprints/BP_EnnemiProjectile.BP_EnnemiProjectile_C" (`SceneComponent.K2_GetComponentToWorld` (`self.SpawnPoint`)) "Undefined" "MultiplyWithRoot" null null)
  (`KismetSystemLibrary.Delay` 0.2)
  (`self.Viser`))

(fn `UserConstructionScript`
  (`parent.UserConstructionScript`))