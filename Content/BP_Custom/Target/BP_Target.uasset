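; BP_Target is a shootable target that notifies linked Portes (doors) when a first-person projectile hits it.
; Its BulletHit event switches on the Actif flag, which arms the collider's overlap response.
; While armed, an overlapping projectile is destroyed and BulletHitMessage is sent to Portes.
; An initially open Gate closes after a hit when DoOnce is set, making the target single-use.
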(event `/Game/BP_Interface/BPI_BulletHit.BulletHit`
  (if (not (`self.Actif`))
    (set `self.Actif` true)))

(event `self.Collider.OnComponentBeginOverlap`
  (params (OverlappedComponent :type "PrimitiveComponent Object Reference") (OtherActor :type "Actor Object Reference") (OtherComp :type "PrimitiveComponent Object Reference") (OtherBodyIndex :type Integer) (bFromSweep :type Boolean) (SweepResult :type "HitResult Structure (by ref)"))
  (if (`self.Actif`)
    (`/Engine/EditorBlueprintResources/StandardMacros.Gate` false :!label _label
      (:`Exit`
        (bind _asbp_first_person_projectile (cast `/Game/FirstPerson/Blueprints/BP_FirstPersonProjectile` OtherActor))
        (`/Game/FirstPerson/Blueprints/BP_FirstPersonProjectile.Destroy` _asbp_first_person_projectile)
        (message `/Game/BP_Interface/BPI_BulletHit.BulletHit` (`self.Portes`))
        (if (`self.DoOnce`)
          (goto _label :!via `Close`))))))

(fn `UserConstructionScript`)