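; BP_ActiveLight is an environment light that shows its point light only when every linked element in Portes is active.
; On BulletHit it opens a Gate immediately, then checks the Portes array after a short delay.
; Any inactive element hides the light and closes the Gate, so the pass after the loop turns the light on only if none were inactive.
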(event `/Game/BP_Interface/BPI_BulletHit.BulletHit`
  (`|ExecutionSequence`
    (:`then_0`
      (goto _label :!via `Break`))
    (:`then_1`
      (`KismetSystemLibrary.Delay` 0.2)
      (for _array_element (`self.Portes`) :!label _label
        (if (not (`/Game/Enviro/BP_ActivableParent.Actif` _array_element))
          (`SceneComponent.SetVisibility` (`self.PointLight`) false false)
          (goto _label_2 :!via `Close`)))
      (`/Engine/EditorBlueprintResources/StandardMacros.Gate` true :!label _label_2
        (:`Exit`
          (`SceneComponent.SetVisibility` (`self.PointLight`) true false))))
    (:`then_2`
      (goto _label_2 :!via `Open`))))

(fn `UserConstructionScript`)