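; Bullet-activated light that turns on when all linked Portes are active, optionally moving a door mesh.
; BulletHit waits briefly, then scans Portes, hiding the PointLight and closing a Gate if any is inactive.
; An open Gate shows the light, clears DoOnce to lock further hits, and, if SMPorte is set, runs a Timeline lerp from the start position to TargetPosition.
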(event `self.ReceiveBeginPlay`
  (bind _sm_porte (`self.SM_Porte`))
  (set `self.BasePosition` (`SceneComponent.K2_GetComponentLocation` (`self.DefaultSceneRoot`)))
  (`/Engine/EditorBlueprintResources/StandardMacros.IsValid` _sm_porte
    (:`Is Valid`
      (`StaticMeshComponent.SetStaticMesh` (`self.StaticMesh`) _sm_porte))))

(event `/Game/BP_Interface/BPI_BulletHit.BulletHit`
  (if (`self.DoOnce`)
    (`|ExecutionSequence`
      (:`then_0`
        (goto _label :!via `Break`))
      (:`then_1`
        (`KismetSystemLibrary.Delay` 0.2)
        (for _array_element (`self.Portes`) :!label _label
          (if (not (`/Game/Enviro/BP_ActivableParent.Actif` _array_element))
            (`SceneComponent.SetVisibility` (`self.PointLight`) false false)
            (goto _label_2 :!via `Close`)))
        (`/Engine/EditorBlueprintResources/StandardMacros.Gate` true :!label _label_2
          (:`Exit`
            (`SceneComponent.SetVisibility` (`self.PointLight`) true false)
            (set `self.DoOnce` false)
            (`/Engine/EditorBlueprintResources/StandardMacros.IsValid` (`self.SM_Porte`)
              (:`Is Valid`
                (`self.MoveSelf`))))))
      (:`then_2`
        (goto _label_2 :!via `Open`)))))

(event `MoveSelf`
  (`KismetSystemLibrary.PrintString` "Hello")
  (bind (_direction _newtrack_0) (`Timeline|Timeline`)
    (:`Update`
      (`SceneComponent.K2_SetWorldLocation` (`self.DefaultSceneRoot`) (`KismetMathLibrary.VLerp` (`self.BasePosition`) (`self.TargetPosition`) _newtrack_0) false false))))

(fn `UserConstructionScript`)